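; Room graph component for the dungeon generator that tracks which rooms connect to each other.
; It stores connections as room pairs in RoomConnections, mirrors them in each room's ConnectedRooms, and offers add, remove, clear and query functions.
; Inserting a room builds candidate links to other rooms, keeping only those without a shorter candidate within 90 degrees, tested by dot product.
; Debug helpers draw connection lines and print the pairs.
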(fn InsertNewRoominGraph
  (params (NewRoom :type Room%20Object%20Reference) (Rooms :type Array%20of%20Room%20Object%20References))
  (bind _localroomconnections (LocalVariables|GetLOCALRoomConnections))
  (for _array_element Rooms
    (bind _output_get (LocalVariables|SetLOCALCurrentRoom _array_element))
    (if (!= _output_get NewRoom)
      (LocalVariables|SetLOCALConnectionAlreadyExists false)
      (bind _array_element_2 (Utilities|Array|ForEachLoopwithBreak (Variables|/Game/DungeonGenerator/Blueprints/Room/Room.Room_C|GetConnectedRooms (LocalVariables|GetLOCALCurrentRoom)) :!label _label)
        (:LoopBody
          (if (== _array_element_2 NewRoom)
            (LocalVariables|SetLOCALConnectionAlreadyExists true)
            (goto _label Break)))
        (:Completed
          (if (not (LocalVariables|GetLOCALConnectionAlreadyExists))
            (Utilities|Array|Add (LocalVariables|GetLOCALRoomConnections) (Utilities|Struct|MakeRoomConnexion (LocalVariables|GetLOCALCurrentRoom) NewRoom)))))))
  ;[1 1 1] Connection filtering : If a connection is clother and in the same direction as the current connection, we don't keep this connection
  (for _array_element_3 _localroomconnections
    (LocalVariables|SetLOCALCurrentConnectionLink (- (Transformation|GetActorLocation (.Room01 (Utilities|Struct|BreakRoomConnexion _array_element_3))) (Transformation|GetActorLocation (.Room02 (Utilities|Struct|BreakRoomConnexion _array_element_3)))))
    (LocalVariables|SetLOCALAddConnection true)
    (bind _array_element_4 (Utilities|Array|ForEachLoopwithBreak _localroomconnections :!label _label_2)
      (:LoopBody
        (if (not (and (== (.Room01 (Utilities|Struct|BreakRoomConnexion _array_element_4)) (.Room01 (Utilities|Struct|BreakRoomConnexion _array_element_3))) (== (.Room02 (Utilities|Struct|BreakRoomConnexion _array_element_4)) (.Room02 (Utilities|Struct|BreakRoomConnexion _array_element_3)))))
          (LocalVariables|SetLOCALTestedConnectionLink (- (Transformation|GetActorLocation (.Room01 (Utilities|Struct|BreakRoomConnexion _array_element_4))) (Transformation|GetActorLocation (.Room02 (Utilities|Struct|BreakRoomConnexion _array_element_4)))))
          (if (and (> (Math|Vector|DotProduct (LocalVariables|GetLOCALCurrentConnectionLink) (LocalVariables|GetLOCALTestedConnectionLink)) 0.0) (< (Math|Vector|VectorLength (LocalVariables|GetLOCALTestedConnectionLink)) (Math|Vector|VectorLength (LocalVariables|GetLOCALCurrentConnectionLink))))
            (LocalVariables|SetLOCALAddConnection false)
            (goto _label_2 Break))))
      (:Completed
        (if (LocalVariables|GetLOCALAddConnection)
          (CallFunction|AddConnectionBetweenRooms (.Room01 (Utilities|Struct|BreakRoomConnexion _array_element_3)) (.Room02 (Utilities|Struct|BreakRoomConnexion _array_element_3)))
          (Math|Integer|IncrementInt (LocalVariables|GetLOCALGeneratedConnectionCount)
            (:%20%20
              (Utilities|Array|Add (LocalVariables|GetLOCALGeneratedRoomConnections) _array_element_3)))))))
  (return (LocalVariables|GetLOCALGeneratedConnectionCount) (LocalVariables|GetLOCALGeneratedRoomConnections)))

(fn AddConnectionBetweenRooms
  (params (Room01 :type Room%20Object%20Reference) (Room02 :type Room%20Object%20Reference))
  (if (Math|Boolean|ANDBoolean (Utilities|IsValid Room01) (Utilities|IsValid Room02) (!= Room01 Room02))
    (Utilities|Array|Add (Variables|Default|GetRoomConnections) (Utilities|Struct|MakeRoomConnexion Room01 Room02))
    (Utilities|Array|Add (Variables|/Game/DungeonGenerator/Blueprints/Room/Room.Room_C|GetConnectedRooms Room01) Room02)
    (Utilities|Array|Add (Variables|/Game/DungeonGenerator/Blueprints/Room/Room.Room_C|GetConnectedRooms Room02) Room01)))

(fn RemoveConnectionBetweenRooms
  (params (Connection :type Room%20Connexion%20Structure))
  (bind (_room01 _room02) (Utilities|Struct|BreakRoomConnexion Connection))
  (Utilities|Array|RemoveItem (Variables|Default|GetRoomConnections) Connection)
  (Utilities|FlowControl|Sequence
    (:then_0
      (Utilities|IsValid _room01
        (:Is%20Valid
          (Utilities|Array|RemoveItem (Variables|/Game/DungeonGenerator/Blueprints/Room/Room.Room_C|GetConnectedRooms _room01) _room02))))
    (:then_1
      (Utilities|IsValid _room02
        (:Is%20Valid
          (Utilities|Array|RemoveItem (Variables|/Game/DungeonGenerator/Blueprints/Room/Room.Room_C|GetConnectedRooms _room02) _room01))))))

(fn RemoveRoomfromGraph
  (params (Room :type Room%20Object%20Reference))
  (bind _connectedrooms (Variables|/Game/DungeonGenerator/Blueprints/Room/Room.Room_C|GetConnectedRooms Room))
  (bind _roomconnections (Variables|Default|GetRoomConnections))
  (for _array_element _connectedrooms
    (Utilities|IsValid _array_element
      (:Is%20Valid
        (Utilities|Array|RemoveItem (Variables|/Game/DungeonGenerator/Blueprints/Room/Room.Room_C|GetConnectedRooms _array_element) Room))))
  (Utilities|Array|Clear _connectedrooms)
  (bind (_arrayindex _arrayelement) (Utilities|Array|ReverseforEachLoop _roomconnections)
    (:LoopBody
      (if (or (== (.Room01 (Utilities|Struct|BreakRoomConnexion _arrayelement)) Room) (== (.Room02 (Utilities|Struct|BreakRoomConnexion _arrayelement)) Room))
        (Utilities|Array|RemoveIndex _roomconnections _arrayindex)))))

(fn ClearRoomConnections
  (bind _roomconnections (Variables|Default|GetRoomConnections))
  (for _array_element _roomconnections
    (CallFunction|RemoveConnectionBetweenRooms _array_element))
  (Utilities|Array|Clear _roomconnections))

(fn GetConnectedRooms
  (params (Room :type Room%20Content%20Object%20Reference))
  (bind _localconnectedrooms (LocalVariables|GetLOCALConnectedRooms))
  (for _array_element (Variables|Default|GetRoomConnections)
    (if (== (.Room01 (Utilities|Struct|BreakRoomConnexion _array_element)) Room)
      (Utilities|Array|Add _localconnectedrooms (.Room02 (Utilities|Struct|BreakRoomConnexion _array_element)))
      (elif (== (.Room02 (Utilities|Struct|BreakRoomConnexion _array_element)) Room)
        (Utilities|Array|Add _localconnectedrooms (.Room01 (Utilities|Struct|BreakRoomConnexion _array_element))))))
  (return (LocalVariables|GetLOCALConnectedRooms)))

(fn GetRoomConnectionCount
  (params (Room :type Room%20Object%20Reference))
  (bind _localconnectedroomscount (LocalVariables|GetLOCALConnectedRoomsCount))
  (for _array_element (Variables|Default|GetRoomConnections)
    (if (== (.Room01 (Utilities|Struct|BreakRoomConnexion _array_element)) Room)
      (Math|Integer|IncrementInt _localconnectedroomscount)
      (elif (== (.Room02 (Utilities|Struct|BreakRoomConnexion _array_element)) Room)
        (Math|Integer|IncrementInt _localconnectedroomscount))))
  (return (LocalVariables|GetLOCALConnectedRoomsCount)))

(fn DebugDrawOneRoomConnection
  (params (Room :type Room%20Object%20Reference))
  (bind _returnvalue (Math|Random|RandomUnitVector))
  (for _array_element (Variables|Default|GetRoomConnections)
    (if (or (== (.Room01 (Utilities|Struct|BreakRoomConnexion _array_element)) Room) (== (.Room02 (Utilities|Struct|BreakRoomConnexion _array_element)) Room))
      (Utilities|FlowControl|Sequence
        (:then_0
          (Rendering|Debug|DrawDebugLine (Default|GetRoomCenterLocation (.Room01 (Utilities|Struct|BreakRoomConnexion _array_element))) (Default|GetRoomCenterLocation (.Room02 (Utilities|Struct|BreakRoomConnexion _array_element))) (Math|Color|MakeColor (.x _returnvalue) (.y _returnvalue) (.z _returnvalue)) 1e+01 1e+01))
        (:then_1
          (Development|PrintString (Utilities|String|ToString(Text) (Utilities|Text|FormatText "Connection {coIdx} : {room01} connected with {room02}" (LocalVariables|GetLOCALConnectionCount) (Utilities|Text|ToText(Object) (.Room01 (Utilities|Struct|BreakRoomConnexion _array_element))) (Utilities|Text|ToText(Object) (.Room02 (Utilities|Struct|BreakRoomConnexion _array_element))))) true true "(R=0.000000,G=0.660000,B=1.000000,A=1.000000)" 1e+01)
          (Math|Integer|IncrementInt (LocalVariables|GetLOCALConnectionCount))))))
  (Development|PrintString (Utilities|String|Append "Connection count : " (Utilities|String|ToString(Integer) (LocalVariables|GetLOCALConnectionCount)))))

(fn DebugDrawRoomConnections
  (bind _returnvalue (Math|Random|RandomUnitVector))
  (Development|PrintString (Utilities|String|ToString(Text) (Utilities|Text|FormatText "Number of connections : {coNum}" (Utilities|Array|Length (Variables|Default|GetRoomConnections)))) true true "(R=0.000000,G=0.660000,B=1.000000,A=1.000000)" 1e+01)
  (for (_array_element _array_index) (Variables|Default|GetRoomConnections)
    (Utilities|FlowControl|Sequence
      (:then_0
        (Rendering|Debug|DrawDebugLine (+ (Default|GetRoomCenterLocation (.Room01 (Utilities|Struct|BreakRoomConnexion _array_element))) "0, 0,100.000000") (+ (Default|GetRoomCenterLocation (.Room02 (Utilities|Struct|BreakRoomConnexion _array_element))) "0, 0,100.000000") (Math|Color|MakeColor (.x _returnvalue) (.y _returnvalue) (.z _returnvalue)) 1e+01 3e+01))
      (:then_1
        (Development|PrintString (Utilities|String|ToString(Text) (Utilities|Text|FormatText "Connection {coIdx} : {room01} connected with {room02}" _array_index (Utilities|Text|ToText(Object) (.Room01 (Utilities|Struct|BreakRoomConnexion _array_element))) (Utilities|Text|ToText(Object) (.Room02 (Utilities|Struct|BreakRoomConnexion _array_element))))) true true "(R=0.000000,G=0.660000,B=1.000000,A=1.000000)" 1e+01)))))

(fn DoesConnectionExistsBetweenRooms
  (params (Room01 :type Room%20Object%20Reference) (Room02 :type Room%20Object%20Reference))
  (for _array_element (Variables|Default|GetRoomConnections)
    (if (or (and (== (.Room01 (Utilities|Struct|BreakRoomConnexion _array_element)) Room01) (== (.Room02 (Utilities|Struct|BreakRoomConnexion _array_element)) Room02)) (and (== (.Room02 (Utilities|Struct|BreakRoomConnexion _array_element)) Room01) (== (.Room01 (Utilities|Struct|BreakRoomConnexion _array_element)) Room02)))
      (return true)))
  (return false))