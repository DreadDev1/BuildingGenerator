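; Editor-placeable guide actor for the dungeon generator that marks a path's two endpoints with a spline and Begin/End markers.
; The construction script snaps Begin to the last spline point and End to the first, and getters expose their world locations.
; Editor functions destroy it, duplicate it through the PathManager, or have the generator regenerate its path.
; Destruction unregisters it from the manager and destroys its TargetedPath.
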(event EventDestroyed
  (bind _pathmanagerref (Variables|Default|GetPathManagerRef))
  (bind _targetedpath (Variables|Default|GetTargetedPath))
  (Utilities|IsValid _pathmanagerref
    (:Is%20Valid
      (Utilities|Array|RemoveItem (Variables|/Game/DungeonGenerator/Blueprints/Paths/DungeonPathManager.DungeonPathManager_C|GetPathGuides _pathmanagerref) self)
      (Utilities|IsValid _targetedpath
        (:Is%20Valid
          (Actor|DestroyActor _targetedpath))))))

(event EventTick
  (params (DeltaSeconds :type Float%20%28single-precision%29)))

(fn ConstructionScript
  (bind _spline (Variables|Default|GetSpline))
  (if (and (Utilities|IsValid (Variables|Default|GetBegin)) (Utilities|IsValid (Variables|Default|GetEnd)))
    (Transformation|SetRelativeLocation (Variables|Default|GetBegin) (Spline|GetLocationatSplinePoint _spline (Spline|GetNumberOfSplinePoints _spline) "Local") false false)
    (Transformation|SetRelativeLocation (Variables|Default|GetEnd) (Spline|GetLocationatSplinePoint _spline 0 "Local") false false)))

(fn GetBeginLocation
  (return (Transformation|GetWorldLocation (Variables|Default|GetBegin))))

(fn GetEndLocation
  (return (Transformation|GetWorldLocation (Variables|Default|GetEnd))))

(fn Init
  (params (PathManagerRef :type Dungeon%20Path%20Manager%20Object%20Reference))
  (Variables|Default|SetPathManagerRef PathManagerRef))

(fn EditorDestroy
  (Actor|DestroyActor))

(fn EditorRegeneratePaths
  (bind _pathmanagerref (Variables|Default|GetPathManagerRef))
  (Utilities|IsValid _pathmanagerref
    (:Is%20Valid
      (Default|RegenerateUniquePathfromGuide (Variables|/Game/DungeonGenerator/Blueprints/Paths/DungeonPathManager.DungeonPathManager_C|GetGeneratorRef _pathmanagerref) self))))

(fn EditorDuplicate
  (bind _pathmanagerref (Variables|Default|GetPathManagerRef))
  (Utilities|IsValid _pathmanagerref
    (:Is%20Valid
      (bind _newpathguide (Default|CreatePathGuide _pathmanagerref))
      (Transformation|SetWorldLocation (Variables|PathGuide_C|GetSpline _newpathguide) (Transformation|GetActorLocation) false false)
      (Spline|SetLocationatSplinePoint (Variables|PathGuide_C|GetSpline _newpathguide) 0 (Variables|/Script/Engine.SceneComponent|GetRelativeLocation (Variables|Default|GetBegin)) "Local" true)
      (Spline|SetLocationatSplinePoint (Variables|PathGuide_C|GetSpline _newpathguide) 1 (Variables|/Script/Engine.SceneComponent|GetRelativeLocation (Variables|Default|GetEnd)) "Local" true)
      (Transformation|SetRelativeLocation (Variables|Default|GetBegin) (Spline|GetLocationatSplinePoint (Variables|PathGuide_C|GetSpline _newpathguide) (Spline|GetNumberOfSplinePoints (Variables|PathGuide_C|GetSpline _newpathguide)) "Local") false false)
      (Transformation|SetRelativeLocation (Variables|Default|GetEnd) (Spline|GetLocationatSplinePoint (Variables|PathGuide_C|GetSpline _newpathguide) 0 "Local") false false)
      (Spline|UpdateSpline (Variables|PathGuide_C|GetSpline _newpathguide)))))