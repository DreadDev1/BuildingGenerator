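; Dungeon generator element that spawns, tracks and removes items in the grid cells of its owning Path or ProceduralRoomContent.
; SpawnAndPlaceNewMesh spawns the first item bundle that has count left and passes placement checks, with snapping, then decrements its count.
; RoomItems are spawned first, then validate and generate themselves for path or room, and are destroyed on failure.
; An index map links cells to spawned actors, whose delete flags protect them from non-forced removal.
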(fn DestroyAllMeshesonCells
  (bind _celldatas (Variables|Default|GetCellDatas))
  (for _array_element _celldatas
    (Utilities|FlowControl|Sequence
      (:then_0
        (bind _arrayelement (Utilities|Array|ReverseforEachLoop (.ActorItems (Utilities|Struct|BreakCellDatas _array_element)))
          (:LoopBody
            (Utilities|IsValid (.Actor (Utilities|Struct|BreakActorInCell _arrayelement))
              (:Is%20Valid
                (Actor|DestroyActor (.Actor (Utilities|Struct|BreakActorInCell _arrayelement))))))
          (:Completed
            (Utilities|Array|Clear (.ActorItems (Utilities|Struct|BreakCellDatas _array_element))))))
      (:then_1
        (bind _arrayelement_2 (Utilities|Array|ReverseforEachLoop (.RoomItems (Utilities|Struct|BreakCellDatas _array_element)))
          (:LoopBody
            (Utilities|IsValid (.RoomItem (Utilities|Struct|BreakRoomItemInCell _arrayelement_2))
              (:Is%20Valid
                (Default|Clear (.RoomItem (Utilities|Struct|BreakRoomItemInCell _arrayelement_2)))
                (Actor|DestroyActor (.RoomItem (Utilities|Struct|BreakRoomItemInCell _arrayelement_2))))))
          (:Completed
            (Utilities|Array|Clear (.RoomItems (Utilities|Struct|BreakCellDatas _array_element))))))))
  (Utilities|Array|Clear _celldatas)
  (Utilities|Map|Clear (Variables|Default|GetCellDatasMapping)))

(fn SpawnandPlaceNewMesh
  (params (AvaillableCounts :type Map%20of%20Integers%20to%20Integers) (CellIdx :type Integer) (CellHeight :type Float%20%28double-precision%29) (CellIdxInPath :type Integer) (CellDirection :type CellDirection4%20Enum :default "NewEnumerator0") (PlacementType :type ItemPlacementZone%20Enum :default "NewEnumerator12") (CellIsCorner :type Boolean) (CellSecondaryDirection :type CellDirection4%20Enum :default "NewEnumerator0") (CellIsInternalCorner :type Boolean) (RoomItems :type Array%20of%20Room%20Item%20Bundle%20Spawn%20Info%20Structures) (MeshLocation :type Vector) (MeshRotation :type Rotator) (DistanceToNearestWall :type Integer))
  (bind _cellsize (Utilities|GetCellSize))
  (LocalVariables|SetLOCALCellSize _cellsize)
  ;[1 1 1] Go through bundles
  (bind _keys (Utilities|Map|Keys AvaillableCounts))
  (LocalVariables|SetLOCALItemBundleCount (Utilities|Array|Length _keys))
  (if (> (Utilities|Array|Length _keys) 0)
    (for _index (range 0 (- (LocalVariables|GetLOCALItemBundleCount) 1))
      (bind _output_get (LocalVariables|SetLOCALChoosenItemBundle (Utilities|Array|Get(acopy) _keys (LocalVariables|GetLOCALItemBundleIndex))))
      ;[1 1 1] Check if the spawn probability of the bundle
      (if (> (.Value (Utilities|Map|Find AvaillableCounts _output_get)) 0)
        (LocalVariables|SetLOCALBundleIsSpawned false)
        (for _array_element (.Items (Utilities|Struct|BreakRoomItemBundleSpawnInfo (Utilities|Array|Get(acopy) RoomItems _output_get)))
          ;[1 1 1] We check if we can spawn the item
          (if (CallFunction|ShouldSpawnItem CellIdx (LocalVariables|GetLOCALCellSize) CellDirection (.ForbiddenDirections (Utilities|Struct|BreakRoomItemBundleSpawnInfo (Utilities|Array|Get(acopy) RoomItems _output_get))) (.PlacementPattern (Utilities|Struct|BreakRoomItemBundleSpawnInfo (Utilities|Array|Get(acopy) RoomItems _output_get))) (.Item (Utilities|Struct|BreakRoomItemSpawnInfo _array_element)) (.ItemAsActor (Utilities|Struct|BreakRoomItemSpawnInfo _array_element)))
            (LocalVariables|SetLOCALBundleIsSpawned true)
            (bind _modifiedlocation (CallFunction|PlacementHelperApplySnappingandOffset CellDirection (.SnapMode (Utilities|Struct|BreakRoomItemSpawnInfo _array_element)) (.SnapDirection (Utilities|Struct|BreakRoomItemSpawnInfo _array_element)) MeshLocation (LocalVariables|GetLOCALCellSize) (.HeightOffset (Utilities|Struct|BreakRoomItemSpawnInfo _array_element))))
            ;[1 1 1] Check if we want to spawn an actor or a RoomItem
            (if (Utilities|IsValidClass (.Item (Utilities|Struct|BreakRoomItemSpawnInfo _array_element)))
              ;[1 1 1] Spawn the RoomItem and attach it to the room. We first check if the item can be successfully spawned
              (bind _returnvalue (Game|SpawnActorfromClass (.Item (Utilities|Struct|BreakRoomItemSpawnInfo _array_element)) (Math|Transform|MakeTransform _modifiedlocation MeshRotation "1.000000,1.000000,1.000000") "AlwaysSpawn" "SelectDefaultAtRuntime" 0 0))
              (Utilities|CanbeSpawnedinPathorRoom _returnvalue PlacementType CellIdx CellHeight CellIdxInPath CellDirection CellIsCorner CellSecondaryDirection CellIsInternalCorner DistanceToNearestWall
                (:CanSpawn
                  (Utilities|GenerateinPathorRoom _returnvalue PlacementType CellIdx CellHeight CellIdxInPath CellDirection CellIsCorner CellSecondaryDirection CellIsInternalCorner DistanceToNearestWall
                    (:Success
                      (bind _output (Utilities|GetorAddCellData CellIdx)
                        (:OutputPin
                          (Utilities|Array|Add (.RoomItems (Utilities|Struct|BreakCellDatas _output)) (Utilities|Struct|MakeRoomItemInCell _returnvalue (.CellIdx (Utilities|Struct|BreakCellDatas _output)) (CallFunction|GetDeleteModeforItemPlacement PlacementType)))
                          (Transformation|AttachActorToActor _returnvalue (Components|GetOwner) "None" "KeepWorld" "KeepWorld" "KeepRelative" true))))
                    (:Failure
                      (Default|Clear _returnvalue :!label _label)
                      (Actor|DestroyActor _returnvalue))))
                (:CannotSpawn
                  (goto _label)))
              (else
                ;[1 1 1] Spawn the item actor and attach it to the room
                (bind _returnvalue_2 (Game|SpawnActorfromClass (.ItemAsActor (Utilities|Struct|BreakRoomItemSpawnInfo _array_element)) (Math|Transform|MakeTransform _modifiedlocation MeshRotation "1.000000,1.000000,1.000000") "AlwaysSpawn" "SelectDefaultAtRuntime" 0 0))
                (bind _output_2 (Utilities|GetorAddCellData CellIdx)
                  (:OutputPin
                    (Utilities|Array|Add (.ActorItems (Utilities|Struct|BreakCellDatas _output_2)) (Utilities|Struct|MakeActorInCell _returnvalue_2 (.CellIdx (Utilities|Struct|BreakCellDatas _output_2)) (CallFunction|GetDeleteModeforItemPlacement PlacementType)))
                    (Transformation|AttachActorToActor _returnvalue_2 (Components|GetOwner) "None" "KeepWorld" "KeepWorld" "KeepRelative" true)))))))
        ;[1 1 1] Once the items have been spawned inside the cell, we reduce the item count
        (if (LocalVariables|GetLOCALBundleIsSpawned)
          (CallFunction|PlacementHelperDecreaseItemCount AvaillableCounts (LocalVariables|GetLOCALChoosenItemBundle))
          (return)
          (else
            (Math|Integer|IncrementInt (LocalVariables|GetLOCALItemBundleIndex))))))))

(fn Init
  (bind _returnvalue (Components|GetOwner))
  (bind _aspath (Utilities|Casting|CastToPath _returnvalue)
    (:then
      (Variables|Default|SetOwnerAsPath _aspath))
    (:CastFailed
      (bind _asprocedural_room_content (Utilities|Casting|CastToProceduralRoomContent _returnvalue))
      (Variables|Default|SetOwnerAsRoomContent _asprocedural_room_content))))

(fn RemoveMeshesinCell
  (params (CellIdx :type Integer) (ForceDelete :type Boolean))
  (bind _output (Utilities|GetCellData CellIdx)
    (:CellFound
      (Utilities|FlowControl|Sequence
        (:then_0
          (bind (_arrayindex _arrayelement) (Utilities|Array|ReverseforEachLoop (.ActorItems (Utilities|Struct|BreakCellDatas _output)))
            (:LoopBody
              (if (or (not (.NeedForceDelete (Utilities|Struct|BreakActorInCell _arrayelement))) (and (.NeedForceDelete (Utilities|Struct|BreakActorInCell _arrayelement)) ForceDelete))
                (Actor|DestroyActor (.Actor (Utilities|Struct|BreakActorInCell _arrayelement)))
                (Utilities|Array|RemoveIndex (.ActorItems (Utilities|Struct|BreakCellDatas _output)) _arrayindex)))))
        (:then_1
          (bind (_arrayindex_2 _arrayelement_2) (Utilities|Array|ReverseforEachLoop (.RoomItems (Utilities|Struct|BreakCellDatas _output)))
            (:LoopBody
              (if (or (not (.NeedHardDelete (Utilities|Struct|BreakRoomItemInCell _arrayelement_2))) (and (.NeedHardDelete (Utilities|Struct|BreakRoomItemInCell _arrayelement_2)) ForceDelete))
                (Default|Clear (.RoomItem (Utilities|Struct|BreakRoomItemInCell _arrayelement_2)))
                (Actor|DestroyActor (.RoomItem (Utilities|Struct|BreakRoomItemInCell _arrayelement_2)))
                (Utilities|Array|RemoveIndex (.RoomItems (Utilities|Struct|BreakCellDatas _output)) _arrayindex_2)))))))))