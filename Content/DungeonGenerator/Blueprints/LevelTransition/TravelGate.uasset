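; Level transition gate that sends a player-controlled pawn entering its Box trigger to a named gate in another level through a TravelManager.
; Register stores the manager, adds the gate to its list and looks up the destination level and gate by GateName.
; Registration also spawns a PlayerStart, if none is set, at the Start component.
; The construction script places Start relative to the Box's forward and up vectors, as the arrival point.
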(event OnComponentBeginOverlap(Box)
  (params (OverlappedComponent :type Primitive%20Component%20Object%20Reference) (OtherActor :type Actor%20Object%20Reference) (OtherComp :type Primitive%20Component%20Object%20Reference) (OtherBodyIndex :type Integer) (bFromSweep :type Boolean) (SweepResult :type Hit%20Result%20Structure%20%28by%20ref%29))
  (bind _aspawn (Utilities|Casting|CastToPawn OtherActor))
  (if (Pawn|IsPlayerControlled _aspawn)
    (bind _asplayer_controller (Utilities|Casting|CastToPlayerController (Pawn|GetController _aspawn)))
    (CallFunction|TraveltoNextLevel _asplayer_controller)))

(fn ConstructionScript
  (bind _box (Variables|Default|GetBox))
  (bind _returnvalue (Components|Box|GetScaledBoxExtent _box))
  (bind _returnvalue_2 (* _returnvalue 0.5))
  (Transformation|SetWorldLocation (Variables|Default|GetStart) (+ (Transformation|GetWorldLocation _box) (* (Math|Vector|GetForwardVector _box) (+ (.x _returnvalue_2) 1e+02)) (* (Math|Vector|GetUpVector _box) (+ (* (.z _returnvalue_2) -1.0) 1.5e+02))) false false))

(fn TraveltoNextLevel
  (params (PlayerController :type Player%20Controller%20Object%20Reference))
  (bind _travelmanager (Variables|Default|GetTravelManager))
  (Utilities|IsValid _travelmanager
    (:Is%20Valid
      (Default|MakePlayerTravel _travelmanager (Utilities|Struct|MakeGateDestinationInfo (Variables|Infos|GetNextLevel) (Variables|Infos|GetNextGate)) PlayerController (Variables|Infos|GetGateName)))))

(fn Init
  (bind _start (Variables|Default|GetStart))
  (Utilities|IsValid (Variables|Default|GetStartAsPlayerStart)
    (:Is%20Not%20Valid
      (bind _returnvalue (Game|SpawnActorfromClass "/Script/Engine.PlayerStart" (Math|Transform|MakeTransform (Transformation|GetWorldLocation _start) (Transformation|GetWorldRotation _start) "1.000000,1.000000,1.000000") "AdjustIfPossibleButAlwaysSpawn" "MultiplyWithRoot" 0 0))
      (Variables|Default|SetStartAsPlayerStart _returnvalue))))

(fn Register
  (params (TravelManager :type Travel%20Manager%20Component%20Object%20Reference))
  (bind _gatename (Variables|Infos|GetGateName))
  (bind _output_get (Variables|Default|SetTravelManager TravelManager))
  (CallFunction|Init)
  (bind _returnvalue (Utilities|Array|AddUnique (Variables|/Game/DungeonGenerator/Blueprints/LevelTransition/TravelManagerComponent.TravelManagerComponent_C|GetLevelGates _output_get) self))
  (if (>= _returnvalue 0)
    (if (.InfosFound (Default|GetGateDestinationInfos _output_get _gatename))
      (Variables|Infos|SetNextLevel (.DestinationLevelName (Utilities|Struct|BreakGateDestinationInfo (.Infos (Default|GetGateDestinationInfos _output_get _gatename)))))
      (Variables|Infos|SetNextGate (.DestinationGateName (Utilities|Struct|BreakGateDestinationInfo (.Infos (Default|GetGateDestinationInfos _output_get _gatename)))))
      (else
        (Development|PrintString (Utilities|String|Append "gate not found : " _gatename))))))