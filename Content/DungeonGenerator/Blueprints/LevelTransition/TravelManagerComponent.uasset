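; Travel manager component that moves players between named travel gates, within a level or across levels.
; Init loads each gate's destination from a data table row, and gates register through an interface scan and a class scan.
; Travel fires a pre-travel callback and stops movement, then teleports within the same level or opens the target level with the gate name as an option.
; Teleporting falls back to the first registered gate if the name is missing.
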(fn FindandRegisterAllGates
  (Utilities|Array|Clear (Variables|Runtime|GetLevelGates))
  (Utilities|FlowControl|Sequence
    (:then_0
      (bind _outactors (Actor|GetAllActorswithInterface "/Game/DungeonGenerator/Blueprints/LevelTransition/ITravelGateOwner.ITravelGateOwner_C"))
      (for _array_element _outactors
        (bind _travelgates (Class|ITravelGateOwner|GetOwnedTravelGates(Message) _array_element))
        (for _array_element_2 _travelgates
          (Default|Register _array_element_2 self))))
    (:then_1
      (bind _outactors_2 (Actor|GetAllActorsOfClass "/Game/DungeonGenerator/Blueprints/LevelTransition/TravelGate.TravelGate_C"))
      (for _array_element_3 _outactors_2
        (Default|Register _array_element_3 self)))))

(fn TeleporttoGate
  (params (GateName :type String) (Pawn :type Pawn%20Object%20Reference))
  (bind (_found _start) (CallFunction|GetPlayerStart GateName))
  (if _found
    (Transformation|SetActorLocationAndRotation Pawn (Transformation|GetActorLocation _start) (Transformation|GetActorRotation _start))
    (return true)
    (else
      (return false))))

(fn GetPlayerStart
  (params (GateName :type String))
  (bind _levelgates (Variables|Runtime|GetLevelGates))
  (for _array_element _levelgates
    (if (Utilities|Enum|Equal(Enum) (Variables|/Game/DungeonGenerator/Blueprints/LevelTransition/TravelGate.TravelGate_C|GetGateName _array_element) GateName)
      (return true (Variables|/Game/DungeonGenerator/Blueprints/LevelTransition/TravelGate.TravelGate_C|GetStartAsPlayerStart _array_element))))
  (if (> (Utilities|Array|Length _levelgates) 0)
    (return true (Variables|/Game/DungeonGenerator/Blueprints/LevelTransition/TravelGate.TravelGate_C|GetStartAsPlayerStart (Utilities|Array|Get(acopy) _levelgates)))
    (else
      (return false 0))))

(fn GetGateDestinationInfos
  (params (GateName :type String))
  (bind _gatesdestinations (Variables|Infos|GetGatesDestinations))
  (bind (_value _returnvalue) (Utilities|Map|Find _gatesdestinations GateName))
  (return _returnvalue _value))

(fn Init
  (bind _gatetraveldatatable (Variables|Infos|GetGateTravelDataTable))
  (bind _gatesdestinations (Variables|Infos|GetGatesDestinations))
  (Utilities|IsValid _gatetraveldatatable
    (:Is%20Valid
      (bind _returnvalue (Utilities|GetDataTableRow _gatetraveldatatable (Variables|Infos|GetEntryInGateTravelDataTable))
        (:then
          (Utilities|Map|Clear _gatesdestinations)
          (bind _keys (Utilities|Map|Keys (Utilities|Struct|BreakGatesTravelInfo _returnvalue)))
          (bind _values (Utilities|Map|Values (Utilities|Struct|BreakGatesTravelInfo _returnvalue)))
          (for (_array_element _array_index) _keys
            (Utilities|Map|Add _gatesdestinations _array_element (Utilities|Array|Get(acopy) _values _array_index))))))))

(fn MakePlayerTravel
  (params (DestinationInfo :type Gate%20Destination%20Info%20Structure) (Player :type Player%20Controller%20Object%20Reference) (FromGate :type String))
  (bind (_destinationlevelname _destinationgatename) (Utilities|Struct|BreakGateDestinationInfo DestinationInfo))
  (LocalVariables|SetLOCALNextLevel _destinationlevelname)
  (bind _output_get (LocalVariables|SetLOCALNextGate _destinationgatename))
  (if (Utilities|Enum|NotEqual(Enum) _output_get "")
    (bind _returnvalue (Game|GetCurrentLevelName true))
    (if (or (Utilities|Enum|Equal(Enum) _returnvalue (LocalVariables|GetLOCALNextLevel)) (Utilities|Enum|Equal(Enum) (LocalVariables|GetLOCALNextLevel) ""))
      (Default|CallOnBeforeTravel Player FromGate DestinationInfo)
      (AI|Navigation|StopMovement Player)
      (bind _success (CallFunction|TeleporttoGate (LocalVariables|GetLOCALNextGate) (Pawn|GetControlledPawn Player)))
      (return _success)
      (else
        (Default|CallOnBeforeTravel Player FromGate DestinationInfo)
        (AI|Navigation|StopMovement Player)
        (Game|OpenLevel(byName) (Utilities|String|StringToName (LocalVariables|GetLOCALNextLevel)) true (Utilities|String|Append "gateName=" (LocalVariables|GetLOCALNextGate)))
        (return true)))
    (else
      (return false))))

(fn UnregisterAllGates
  (Utilities|Array|Clear (Variables|Runtime|GetLevelGates)))